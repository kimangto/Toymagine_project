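; BP_WindSpaceTriggerVolume is a wind trigger volume meant to push BP_TestEscapePlayerCharacter along world +Y.
; BeginPlay caches the player character, and WIndForceToPlayer applies a single AddForce scaled by WindForce to its movement component per call.
; A custom overlap handler calls that function for the player character, but its binding node is never executed and the built-in overlap and Tick events are empty.
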(event Custom|OnActorBeginOverlap_Event
  (params (OverlappedActor :type Actor%20Object%20Reference) (OtherActor :type Actor%20Object%20Reference))
  (bind _asbp_test_escape_player_character (Utilities|Casting|CastToBP_TestEscapePlayerCharacter OtherActor))
  (Utilities|IsValid _asbp_test_escape_player_character
    (:Is%20Valid
      (CallFunction|WIndForcetoPlayer))))

(event EventBeginPlay
  (bind _asbp_test_escape_player_character (Utilities|Casting|CastToBP_TestEscapePlayerCharacter (Game|Player|GetPlayerPawn 0)))
  (Utilities|IsValid _asbp_test_escape_player_character
    (:Is%20Valid
      (Variables|Default|SetAs%20BP%20Test%20Escape%20Player%20Character _asbp_test_escape_player_character))))

(event Collision|EventActorBeginOverlap
  (params (OtherActor :type Actor%20Object%20Reference)))

(event EventTick
  (params (DeltaSeconds :type Float%20%28single-precision%29)))

(fn ConstructionScript)

(fn WIndForcetoPlayer
  (bind _output_get (Variables|Default|SetWindDirection "0.000000,1.000000,0.000000"))
  (Physics|AddForce (Variables|/Script/Engine.Character|GetCharacterMovement (Variables|Default|GetAs%20BP%20Test%20Escape%20Player%20Character)) (* _output_get (Variables|Default|GetWindForce))))