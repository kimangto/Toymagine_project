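; Wind zone actor that pushes the BP_TestEscapePlayerCharacter player while they stand inside its WindSpace volume.
; BeginPlay caches the player, and overlap begin and end toggle a flag that gates a per-Tick impulse along world +Y, scaled by WindForce but not by delta time.
; Entering also lowers walking braking deceleration and max acceleration so the wind can move the player, and leaving sets both to very high hardcoded values.
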(event OnComponentBeginOverlap(WindSpace)
  (params (OverlappedComponent :type Primitive%20Component%20Object%20Reference) (OtherActor :type Actor%20Object%20Reference) (OtherComp :type Primitive%20Component%20Object%20Reference) (OtherBodyIndex :type Integer) (bFromSweep :type Boolean) (SweepResult :type Hit%20Result%20Structure%20%28by%20ref%29))
  (bind _as_bp_test_escape_player_character (Variables|Default|GetAs%20BP%20Test%20Escape%20Player%20Character))
  (bind _charactermovement (Variables|/Script/Engine.Character|GetCharacterMovement _as_bp_test_escape_player_character))
  (bind _asbp_test_escape_player_character (Utilities|Casting|CastToBP_TestEscapePlayerCharacter OtherActor))
  (Utilities|IsValid _asbp_test_escape_player_character
    (:Is%20Valid
      (Variables|Default|SetIsInPlayer true)
      (Variables|/Script/Engine.CharacterMovementComponent|SetBrakingDecelerationWalking _charactermovement 3e+02)
      (Variables|/Script/Engine.CharacterMovementComponent|SetMaxAcceleration _charactermovement 1e+03))))

(event OnComponentEndOverlap(WindSpace)
  (params (OverlappedComponent :type Primitive%20Component%20Object%20Reference) (OtherActor :type Actor%20Object%20Reference) (OtherComp :type Primitive%20Component%20Object%20Reference) (OtherBodyIndex :type Integer))
  (bind _as_bp_test_escape_player_character (Variables|Default|GetAs%20BP%20Test%20Escape%20Player%20Character))
  (bind _charactermovement (Variables|/Script/Engine.Character|GetCharacterMovement _as_bp_test_escape_player_character))
  (bind _asbp_test_escape_player_character (Utilities|Casting|CastToBP_TestEscapePlayerCharacter OtherActor))
  (Utilities|IsValid _asbp_test_escape_player_character
    (:Is%20Valid
      (Variables|Default|SetIsInPlayer false)
      (Variables|/Script/Engine.CharacterMovementComponent|SetBrakingDecelerationWalking _charactermovement 999999.0)
      (Variables|/Script/Engine.CharacterMovementComponent|SetMaxAcceleration _charactermovement 999999.0))))

(event EventBeginPlay
  (bind _asbp_test_escape_player_character (Utilities|Casting|CastToBP_TestEscapePlayerCharacter (Game|Player|GetPlayerPawn 0)))
  (Utilities|IsValid _asbp_test_escape_player_character
    (:Is%20Valid
      (Variables|Default|SetAs%20BP%20Test%20Escape%20Player%20Character _asbp_test_escape_player_character))))

(event Collision|EventActorBeginOverlap
  (params (OtherActor :type Actor%20Object%20Reference)))

(event EventTick
  (params (DeltaSeconds :type Float%20%28single-precision%29))
  (if (Variables|Default|GetIsInPlayer)
    (CallFunction|WIndForcetoPlayer)))

(fn ConstructionScript)

(fn WIndForcetoPlayer
  (bind _output_get (Variables|Default|SetWind%20Direction "0.000000,1.000000,0.000000"))
  (Physics|AddImpulse (Variables|/Script/Engine.Character|GetCharacterMovement (Variables|Default|GetAs%20BP%20Test%20Escape%20Player%20Character)) (* _output_get (Variables|Default|GetWind%20Force)) false))