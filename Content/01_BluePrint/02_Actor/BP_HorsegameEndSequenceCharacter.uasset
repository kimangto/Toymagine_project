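; Skeletal mesh stand-in for the horse game's end sequence, kept hidden until the ending starts.
; BeginPlay hides the mesh and caches the player pawn as BP_HorsePlayerCharacter.
; Tick polls that character's IsEndingSequence flag, then clears it and reveals the mesh, so the flag acts as a one-shot trigger.
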(event EventBeginPlay
  (Development|SetHiddeninGame (Variables|SkeletalMeshActor|GetSkeletalMeshComponent) true false)
  (bind _asbp_horse_player_character (Utilities|Casting|CastToBP_HorsePlayerCharacter (Game|Player|GetPlayerPawn 0)))
  (Utilities|IsValid _asbp_horse_player_character
    (:Is%20Valid
      (Variables|Default|SetAs%20BP%20Horse%20Player%20Character _asbp_horse_player_character))))

(event Collision|EventActorBeginOverlap
  (params (OtherActor :type Actor%20Object%20Reference)))

(event EventTick
  (params (DeltaSeconds :type Float%20%28single-precision%29))
  (bind _as_bp_horse_player_character (Variables|Default|GetAs%20BP%20Horse%20Player%20Character))
  (if (Variables|/Game/01_BluePrint/01_Character/BP_HorsePlayerCharacter.BP_HorsePlayerCharacter_C|GetisEndingSequence _as_bp_horse_player_character)
    (Variables|/Game/01_BluePrint/01_Character/BP_HorsePlayerCharacter.BP_HorsePlayerCharacter_C|SetisEndingSequence _as_bp_horse_player_character false)
    (Development|SetHiddeninGame (Variables|SkeletalMeshActor|GetSkeletalMeshComponent) false false)))

(fn ConstructionScript)