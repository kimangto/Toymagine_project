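; BP_RandomCarrotSpawner is a horse game item actor that spawns a single BP_Carrot at a random sideways position when play begins.
; BeginPlay divides Width into eighths, storing eight evenly spaced Y offsets from just inside the negative half-width up to the positive half-width.
; One random offset is added to the StaticMesh's world Y, keeping its rotation, so placement follows the world axis regardless of spawner orientation.
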(event EventBeginPlay
  (bind _width (Variables|Default|GetWidth))
  (bind _staticmesh (Variables|Default|GetStaticMesh))
  (bind _returnvalue (Transformation|GetWorldTransform _staticmesh))
  (Variables|Default|SetDivideWidth (/ (* _width -1.0) 2.0))
  (for _index (range 0 7)
    (bind _output_get (Variables|Default|SetDivideWidth (+ (Variables|Default|GetDivideWidth) (/ _width 8.0))))
    (Utilities|Array|Add (Variables|Default|GetYposition) _output_get))
  (Game|SpawnActorfromClass "/Game/01_BluePrint/02_Actor/01_Item/HorseGameItem/BP_Carrot.BP_Carrot_C" (Math|Transform|MakeTransform (Math|Vector|MakeVector (.x (.location _returnvalue)) (+ (.y (.location _returnvalue)) (.OutItem (Utilities|Array|Random (Variables|Default|GetYposition)))) (.z (.location _returnvalue))) (.rotation _returnvalue) "1.000000,1.000000,1.000000") "Undefined" "MultiplyWithRoot" 0 0))

(event Collision|EventActorBeginOverlap
  (params (OtherActor :type Actor%20Object%20Reference)))

(event EventTick
  (params (DeltaSeconds :type Float%20%28single-precision%29)))

(fn ConstructionScript)