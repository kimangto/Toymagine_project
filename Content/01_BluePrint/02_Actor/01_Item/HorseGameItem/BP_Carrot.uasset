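; BP_Carrot is a horse-game pickup that puts the player's horse character into Fever.
; Tick bobs the static mesh up and down between fixed relative Z limits by flipping a direction flag, while slowly spinning its yaw.
; When BP_HorsePlayerCharacter overlaps the mesh, the carrot sets IsFever, resets FeverTime to zero and destroys itself.
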(event OnComponentBeginOverlap(StaticMesh)
  (params (OverlappedComponent :type Primitive%20Component%20Object%20Reference) (OtherActor :type Actor%20Object%20Reference) (OtherComp :type Primitive%20Component%20Object%20Reference) (OtherBodyIndex :type Integer) (bFromSweep :type Boolean) (SweepResult :type Hit%20Result%20Structure%20%28by%20ref%29))
  (bind _asbp_horse_player_character (Utilities|Casting|CastToBP_HorsePlayerCharacter OtherActor))
  (Variables|/Game/01_BluePrint/01_Character/BP_HorsePlayerCharacter.BP_HorsePlayerCharacter_C|SetisFever _asbp_horse_player_character true)
  (Variables|/Game/01_BluePrint/01_Character/BP_HorsePlayerCharacter.BP_HorsePlayerCharacter_C|SetFeverTime _asbp_horse_player_character 0.0)
  (Actor|DestroyActor))

(event EventBeginPlay
  (Variables|Default|SetUpperZPosition 2e+01)
  (Variables|Default|SetUnderZPosition -2e+01))

(event Collision|EventActorBeginOverlap
  (params (OtherActor :type Actor%20Object%20Reference)))

(event EventTick
  (params (DeltaSeconds :type Float%20%28single-precision%29))
  (bind _staticmesh (Variables|Default|GetStaticMesh))
  (bind _staticmesh_2 (Variables|Default|GetStaticMesh))
  (bind _relativelocation (Variables|/Script/Engine.SceneComponent|GetRelativeLocation _staticmesh))
  (bind _relativelocation_2 (Variables|/Script/Engine.SceneComponent|GetRelativeLocation _staticmesh_2))
  (Utilities|FlowControl|Sequence
    (:then_0
      (if (Variables|Default|GetisUpperZPosition)
        (Variables|Default|SetCarrot%20Location%20Z (- (.z _relativelocation) (* DeltaSeconds 1e+01)))
        (Transformation|SetRelativeLocation _staticmesh (Math|Vector|MakeVector (.x _relativelocation) (.y _relativelocation) (Variables|Default|GetCarrot%20Location%20Z)) false false)
        (if (<= (Variables|Default|GetCarrot%20Location%20Z) (Variables|Default|GetUnderZPosition))
          (Variables|Default|SetisUpperZPosition false))
        (else
          (Variables|Default|SetCarrot%20Location%20Z (+ (.z _relativelocation_2) (* DeltaSeconds 1e+01)))
          (Transformation|SetRelativeLocation _staticmesh_2 (Math|Vector|MakeVector (.x _relativelocation_2) (.y _relativelocation_2) (Variables|Default|GetCarrot%20Location%20Z)) false false)
          (if (>= (Variables|Default|GetCarrot%20Location%20Z) (Variables|Default|GetUpperZPosition))
            (Variables|Default|SetisUpperZPosition true)))))
    (:then_1
      (bind _output_get (Variables|Default|SetCarrot%20Yaw (+ (Variables|Default|GetCarrot%20Yaw) (* DeltaSeconds 1e+01))))
      (Transformation|SetRelativeRotation (Variables|Default|GetStaticMesh) (Math|Rotator|MakeRotator 0.0 0.0 _output_get) false false))))

(fn ConstructionScript)