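; A flag checkpoint item, apparently for the beanstalk escape minigame, that saves the player's respawn position.
; It caches its own location at BeginPlay.
; When a BP_TestEscapePlayerCharacter overlaps its static mesh, it writes that location, raised slightly on Z, into the character's SaveLocation and plays a congratulation sound.
; An IsSave flag makes each checkpoint trigger only once.
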(event OnComponentBeginOverlap(StaticMesh)
  (params (OverlappedComponent :type Primitive%20Component%20Object%20Reference) (OtherActor :type Actor%20Object%20Reference) (OtherComp :type Primitive%20Component%20Object%20Reference) (OtherBodyIndex :type Integer) (bFromSweep :type Boolean) (SweepResult :type Hit%20Result%20Structure%20%28by%20ref%29))
  (bind _savelocation (Variables|Default|GetSaveLocation))
  (if (not (Variables|Default|GetisSave))
    (bind _asbp_test_escape_player_character (Utilities|Casting|CastToBP_TestEscapePlayerCharacter OtherActor))
    (Utilities|IsValid _asbp_test_escape_player_character
      (:Is%20Valid
        (Variables|/Game/01_BluePrint/01_Character/BP_TestEscapePlayerCharacter.BP_TestEscapePlayerCharacter_C|SetsaveLocation _asbp_test_escape_player_character (Math|Vector|MakeVector (.x _savelocation) (.y _savelocation) (+ (.z _savelocation) 1.5e+02)))
        (Audio|PlaySound2D "/Game/03_Resource/03_Volume/SQ_Congratulation.SQ_Congratulation" 1.0 1.0 0.0 0 0)
        (Variables|Default|SetisSave true)))))

(event EventBeginPlay
  (Variables|Default|SetSaveLocation (Transformation|GetActorLocation)))

(event Collision|EventActorBeginOverlap
  (params (OtherActor :type Actor%20Object%20Reference)))

(event EventTick
  (params (DeltaSeconds :type Float%20%28single-precision%29)))

(fn ConstructionScript)