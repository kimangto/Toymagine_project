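; BP_leaf is a leaf platform with moving, vanishing and spring variants, chosen by variables and color-coded by material at BeginPlay.
; Tick sweeps the leaf between its start and Target positions, swapping endpoints on arrival and optionally pausing two seconds.
; On hit, RemoveLeaf hides mesh and collision after a delay, then restores them, while SpringLeaf launches player 0 with sound.
; Rotation logic is unconnected, and MakeRotate and MakeRemove are empty.
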(event OnComponentHit(leaf)
  (params (HitComponent :type Primitive%20Component%20Object%20Reference) (OtherActor :type Actor%20Object%20Reference) (OtherComp :type Primitive%20Component%20Object%20Reference) (NormalImpulse :type Vector :default "0, 0, 0") (Hit :type Hit%20Result%20Structure%20%28by%20ref%29))
  (Utilities|FlowControl|Sequence
    (:then_0
      (if (Variables|Default|GetRemove_leaf)
        (Utilities|FlowControl|Delay 3.0)
        (Components|StaticMesh|SetStaticMesh (Variables|Default|Getleaf) 0)
        (Collision|SetCollisionEnabled (Variables|Default|Getleaf) "NoCollision")
        (Utilities|FlowControl|Delay 3.0)
        (Components|StaticMesh|SetStaticMesh (Variables|Default|Getleaf) "/Game/02_Assets/A_Beanstalk/Leaves/leaf1.leaf1")
        (Collision|SetCollisionEnabled (Variables|Default|Getleaf) "QueryAndPhysics")))
    (:then_1
      (if (Variables|Default|GetSpring_leaf)
        (Physics|AddImpulse (Variables|/Script/Engine.Character|GetCharacterMovement (Game|GetPlayerCharacter 0)) (Variables|Default|GetSpring_value) true)
        (Audio|PlaySound2D "/Game/03_Resource/03_Volume/SQ_SpringLeaf.SQ_SpringLeaf" 1.0 1.0 0.0 0 0)))))

(event EventBeginPlay
  (Utilities|FlowControl|Sequence
    (:then_0
      (Variables|Default|SetStart_Loca (Variables|/Script/Engine.SceneComponent|GetRelativeLocation (Variables|Default|Getleaf)))
      (Variables|Default|SetTarget_Loca (Variables|/Script/Engine.SceneComponent|GetRelativeLocation (Variables|Default|Gettarget))))
    (:then_1
      (if (Variables|Default|GetRemove_leaf)
        (Rendering|Material|SetMaterial (Variables|Default|Getleaf) 0 "/Game/02_Assets/A_Beanstalk/Leaves/M_leaves_R.M_leaves_R")))
    (:then_2
      (if (Variables|Default|GetSpring_leaf)
        (Rendering|Material|SetMaterial (Variables|Default|Getleaf) 0 "/Game/02_Assets/A_Beanstalk/Leaves/M_leaves_S.M_leaves_S")))
    (:then_3
      (if (> (Variables|Default|GetMoveSpeed) 0.0)
        (Rendering|Material|SetMaterial (Variables|Default|Getleaf) 0 "/Game/02_Assets/A_Beanstalk/Leaves/M_leaves_M.M_leaves_M")))))

(event Collision|EventActorBeginOverlap
  (params (OtherActor :type Actor%20Object%20Reference)))

(event EventTick
  (params (DeltaSeconds :type Float%20%28single-precision%29))
  (if (Variables|Default|GetMove_stay_leaf)
    (CallFunction|MoveStay DeltaSeconds)
    (else
      (CallFunction|DontMoveStay DeltaSeconds))))

(fn ConstructionScript)

(fn MakeMove
  (params (Delta_time :type Float%20%28double-precision%29))
  (Transformation|SetRelativeLocation (Variables|Default|Getleaf) (+ (* (Math|Vector|Normalize (- (Variables|Default|GetTarget_Loca) (Variables|Default|GetStart_Loca))) (* Delta_time (Variables|Default|GetMoveSpeed))) (Variables|/Script/Engine.SceneComponent|GetRelativeLocation (Variables|Default|Getleaf))) true false))

(fn CalculateDistance
  (Variables|Default|SetTotal_distance (Math|Vector|VectorLength (- (Variables|Default|GetTarget_Loca) (Variables|Default|GetStart_Loca))))
  (Variables|Default|SetMoved_distance (Math|Vector|VectorLength (- (Variables|/Script/Engine.SceneComponent|GetRelativeLocation (Variables|Default|Getleaf)) (Variables|Default|GetStart_Loca)))))

(fn PointChange
  (if (>= (Variables|Default|GetMoved_distance) (Variables|Default|GetTotal_distance))
    (Variables|Default|SetTemp_Loca (Variables|Default|GetStart_Loca))
    (Variables|Default|SetStart_Loca (Variables|Default|GetTarget_Loca))
    (Variables|Default|SetTarget_Loca (Variables|Default|GetTemp_Loca))
    (return true)
    (else
      (return false))))

(fn MoveStop
  (params (Delta_time :type Float%20%28double-precision%29))
  (bind _output_get (Variables|Default|SetAcc_time (+ Delta_time (Variables|Default|GetAcc_time))))
  (if (> _output_get 2.0)
    (Variables|Default|SetWait_condition false)
    (Variables|Default|SetAcc_time 0.0)))

(fn MoveStay
  (params (Delta_time :type Float%20%28double-precision%29))
  (if (Variables|Default|GetWait_condition)
    (CallFunction|MoveStop Delta_time)
    (else
      (CallFunction|CalculateDistance)
      (bind _changed (CallFunction|PointChange))
      (Variables|Default|SetWait_condition _changed)
      (CallFunction|MakeMove Delta_time))))

(fn DontMoveStay
  (params (Delta_time :type Float%20%28double-precision%29))
  (CallFunction|CalculateDistance)
  (CallFunction|PointChange)
  (CallFunction|MakeMove Delta_time))

(fn MakeRemove)

(fn MakeRotate
  (params (Delta_time :type Float%20%28double-precision%29)))