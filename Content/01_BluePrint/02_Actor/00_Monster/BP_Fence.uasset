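; BP_Fence is an actor, filed among monsters, with a Bullseye mesh meant to break when hit.
; On hit, it checks that BP_HorsePlayerCharacter is valid and that the player controller's forward vector length exceeds 2000, which a unit vector never does.
; Past that check, it sets the mesh, waits a second, sets it again and disables collision.
; Both mesh inputs are empty, with a note to use a fractured asset.
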(event OnComponentHit(bullseye)
  (params (HitComponent :type Primitive%20Component%20Object%20Reference) (OtherActor :type Actor%20Object%20Reference) (OtherComp :type Primitive%20Component%20Object%20Reference) (NormalImpulse :type Vector :default "0, 0, 0") (Hit :type Hit%20Result%20Structure%20%28by%20ref%29))
  (Utilities|IsValid "/Game/01_BluePrint/01_Character/BP_HorsePlayerCharacter.BP_HorsePlayerCharacter"
    (:Is%20Valid
      (if (> (Math|Vector|VectorLength (Transformation|GetActorForwardVector (Game|GetPlayerController 0))) 2e+03)
        ;[1 1 1] 프랙쳐한 에셋으로 바꿔줘야함
        (Components|StaticMesh|SetStaticMesh (Variables|Default|Getbullseye) 0)
        (Utilities|FlowControl|Delay 1.0)
        (Components|StaticMesh|SetStaticMesh (Variables|Default|Getbullseye) 0)
        (Collision|SetCollisionEnabled (Variables|Default|Getbullseye) "NoCollision")))))

(event EventBeginPlay)

(event Collision|EventActorBeginOverlap
  (params (OtherActor :type Actor%20Object%20Reference)))

(event EventTick
  (params (DeltaSeconds :type Float%20%28single-precision%29)))

(fn ConstructionScript)