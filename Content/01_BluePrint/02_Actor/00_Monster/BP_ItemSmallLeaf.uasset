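; BP_ItemSmallLeaf is a thrown leaf item projectile that turns into a BP_ItemHugeLeaf on contact.
; BeginPlay plays the throw sound and derives a Progression vector from the mesh's relative rotation.
; Tick applies that vector as a repeated impulse and sphere-traces on Visibility at the mesh's relative location.
; A hit spawns the huge leaf at the mesh's world transform and destroys this actor.
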(event EventBeginPlay
  (Audio|PlaySound2D "/Game/03_Resource/03_Volume/SQ_LeafThrow.SQ_LeafThrow" 1.0 1.0 0.0 0 0)
  (Variables|Default|SetProgression (* (* (Variables|/Script/Engine.SceneComponent|GetRelativeRotation (Variables|Default|GetStaticMesh)) "1.000000,1.000000,1.000000") 5e+02)))

(event Collision|EventActorBeginOverlap
  (params (OtherActor :type Actor%20Object%20Reference)))

(event EventTick
  (params (DeltaSeconds :type Float%20%28single-precision%29))
  (bind _staticmesh (Variables|Default|GetStaticMesh))
  (bind _relativelocation (Variables|/Script/Engine.SceneComponent|GetRelativeLocation _staticmesh))
  (Utilities|FlowControl|Sequence
    (:then_0
      (Physics|AddImpulse (Variables|Default|GetStaticMesh) (Variables|Default|GetProgression) "None" false))
    (:then_1
      (bind (_outhit _returnvalue) (Collision|SphereTraceByChannel _relativelocation _relativelocation 8e+01 "TraceTypeQuery1" false 0 "None"))
      (if _returnvalue
        (Game|SpawnActorfromClass "/Game/01_BluePrint/02_Actor/00_Monster/BP_ItemHugeLeaf.BP_ItemHugeLeaf_C" (Transformation|GetWorldTransform (Variables|Default|GetStaticMesh)) "Undefined" "MultiplyWithRoot" 0 0)
        (Actor|DestroyActor)))))

(fn ConstructionScript)