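; BP_BlueBird is a bee-game monster actor that patrols back and forth between its mesh's starting position and a Target component.
; BeginPlay caches both relative locations, the distance between them and the base speed.
; Tick moves the skeletal mesh in a straight line until the traveled distance reaches that length, then pauses it for WaitTime.
; After the wait, it swaps the endpoints, turns the mesh 180 degrees in yaw and resumes.
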(event EventBeginPlay
  (CallFunction|InitBlueBird))

(event Collision|EventActorBeginOverlap
  (params (OtherActor :type Actor%20Object%20Reference)))

(event EventTick
  (params (DeltaSeconds :type Float%20%28single-precision%29))
  (CallFunction|TraveledDistance)
  (CallFunction|ArriveTarget)
  (CallFunction|WaitBirdTime DeltaSeconds)
  (CallFunction|InitWaitTime)
  (CallFunction|MoveUpdate DeltaSeconds))

(fn ConstructionScript)

(fn InitStartLocation
  ;[1 1 1] Start Location 설정
  (Variables|Default|SetStartLocation (Variables|/Script/Engine.SceneComponent|GetRelativeLocation (Variables|Default|GetSkeletalMesh))))

(fn InitTargetLocation
  ;[1 1 1] Target Location 설정
  (Variables|Default|SetTargetLocation (Variables|/Script/Engine.SceneComponent|GetRelativeLocation (Variables|Default|GetTarget))))

(fn RoundTripDistance
  ;[1 1 1] start부터 Target 까지의 거리
  (Variables|Default|SetLength (Math|Vector|VectorLength (- (Variables|Default|GetTargetLocation) (Variables|Default|GetStartLocation)))))

(fn InitBaseSpeed
  ;[1 1 1] BaseSpeed 설정
  (Variables|Default|SetSpeed (Variables|Default|GetBaseSpeed)))

(fn InitBlueBird
  (CallFunction|InitStartLocation)
  (CallFunction|InitTargetLocation)
  (CallFunction|RoundTripDistance)
  (CallFunction|InitBaseSpeed))

(fn TraveledDistance
  ;[1 1 1] 이동한 거리
  (Variables|Default|SetTraveledLength (Math|Vector|VectorLength (- (Variables|/Script/Engine.SceneComponent|GetRelativeLocation (Variables|Default|GetSkeletalMesh)) (Variables|Default|GetStartLocation)))))

(fn ArriveTarget
  ;[1 1 1] 도착지점에 도착했을 때
  (if (>= (Variables|Default|GetTraveledLength) (Variables|Default|GetLength))
    (Variables|Default|SetisFinish true)
    (Variables|Default|SetSpeed 0.0)))

(fn WaitBirdTime
  (params (DeltaTime :type Float%20%28double-precision%29))
  ;[1 1 1] 새 도착후 기다리는 시간
  (if (Variables|Default|GetisFinish)
    (Variables|Default|SetTime (+ (Variables|Default|GetTime) DeltaTime))))

(fn Shuffle
  (Variables|Default|SetTempLocation (Variables|Default|GetStartLocation))
  (Variables|Default|SetStartLocation (Variables|Default|GetTargetLocation))
  (Variables|Default|SetTargetLocation (Variables|Default|GetTempLocation)))

(fn InitWaitTime
  (bind _skeletalmesh (Variables|Default|GetSkeletalMesh))
  (bind _relativerotation (Variables|/Script/Engine.SceneComponent|GetRelativeRotation _skeletalmesh))
  ;[1 1 1] Location Shuffle 및 WaitTime 초기화
  (if (>= (Variables|Default|GetTime) (Variables|Default|GetWaitTime))
    (CallFunction|Shuffle)
    (Transformation|SetRelativeRotation _skeletalmesh (Math|Rotator|MakeRotator (.roll _relativerotation) (.pitch _relativerotation) (+ (.yaw _relativerotation) 1.8e+02)) false false)
    (Variables|Default|SetisFinish false)
    (Variables|Default|SetTime 0.0)
    (Variables|Default|SetSpeed (Variables|Default|GetBaseSpeed))))

(fn MoveUpdate
  (params (DeltaTime :type Float%20%28single-precision%29))
  ;[1 1 1] 이동
  (Transformation|SetRelativeLocation (Variables|Default|GetSkeletalMesh) (+ (Variables|/Script/Engine.SceneComponent|GetRelativeLocation (Variables|Default|GetSkeletalMesh)) (* (Math|Vector|Normalize (- (Variables|Default|GetTargetLocation) (Variables|Default|GetStartLocation))) (* (Variables|Default|GetSpeed) DeltaTime))) false false))