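; BP_MonsterFlower is a flower monster actor in the bee game that switches its attack state when the bee player comes near.
; On BeginPlay it starts an idle montage on the skeletal mesh and caches its ABP_MonsterFlower anim instance.
; The static mesh serves as the trigger: begin and end overlaps with BP_BeePlayerCharacter toggle IsAttack and copy it to the anim blueprint.
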(event OnComponentBeginOverlap(StaticMesh)
  (params (OverlappedComponent :type Primitive%20Component%20Object%20Reference) (OtherActor :type Actor%20Object%20Reference) (OtherComp :type Primitive%20Component%20Object%20Reference) (OtherBodyIndex :type Integer) (bFromSweep :type Boolean) (SweepResult :type Hit%20Result%20Structure%20%28by%20ref%29))
  (bind _asbp_bee_player_character (Utilities|Casting|CastToBP_BeePlayerCharacter OtherActor))
  (Utilities|IsValid _asbp_bee_player_character
    (:Is%20Valid
      (bind _output_get (Variables|Default|SetisAttack true))
      (Variables|/Game/01_BluePrint/02_Actor/00_Monster/BeeGame/MonsterFlower/ABP_MonsterFlower.ABP_MonsterFlower_C|SetisAttack (Variables|Default|GetABPMonsterFlower) _output_get))))

(event OnComponentEndOverlap(StaticMesh)
  (params (OverlappedComponent :type Primitive%20Component%20Object%20Reference) (OtherActor :type Actor%20Object%20Reference) (OtherComp :type Primitive%20Component%20Object%20Reference) (OtherBodyIndex :type Integer))
  (bind _asbp_bee_player_character (Utilities|Casting|CastToBP_BeePlayerCharacter OtherActor))
  (Utilities|IsValid _asbp_bee_player_character
    (:Is%20Valid
      (bind _output_get (Variables|Default|SetisAttack false))
      (Variables|/Game/01_BluePrint/02_Actor/00_Monster/BeeGame/MonsterFlower/ABP_MonsterFlower.ABP_MonsterFlower_C|SetisAttack (Variables|Default|GetABPMonsterFlower) _output_get))))

(event EventBeginPlay
  (Animation|Montage|PlayMontage (Variables|Default|GetSkeletalMesh) "/Game/02_Assets/A_Bee/Bee_MonsterFlower/Amon_MonsterFlowerIdle.Amon_MonsterFlowerIdle"
    (:then
      (bind _asabp_monster_flower (Utilities|Casting|CastToABP_MonsterFlower (Components|SkeletalMesh|GetAnimInstance (Variables|Default|GetSkeletalMesh))))
      (Variables|Default|SetABPMonsterFlower _asabp_monster_flower))))

(event Collision|EventActorBeginOverlap
  (params (OtherActor :type Actor%20Object%20Reference)))

(event EventTick
  (params (DeltaSeconds :type Float%20%28single-precision%29)))

(fn ConstructionScript)