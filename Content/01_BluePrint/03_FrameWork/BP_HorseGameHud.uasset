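; BP_HorseGameHud is the HUD Blueprint for the horse game, managing its main game widget and pause screen.
; On BeginPlay it creates UI_HorseGame for player 0, adds it to the viewport and stores the reference.
; ShowPauseUI_HUD creates UI_Pause on demand, caches it and gives it focus; later calls only make the cached widget visible, without refocusing it.
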(event Custom|ShowPauseUI_HUD
  ;[1 1 1] 퍼즈 유아이
  (Utilities|IsValid (Variables|Default|GetPause%20UI)
    (:Is%20Valid
      (Widget|SetVisibility (Variables|Default|GetPause%20UI) "Visible"))
    (:Is%20Not%20Valid
      (bind _returnvalue (UserInterface|CreateWidget "/Game/01_BluePrint/04_UI/CommonUI/UI_Pause.UI_Pause_C"))
      (bind _output_get (Variables|Default|SetPause%20UI _returnvalue))
      (UserInterface|Viewport|AddtoViewport _output_get 0)
      (Widget|SetFocus (Variables|Default|GetPause%20UI)))))

(event EventBeginPlay
  (bind _returnvalue (UserInterface|CreateWidget "/Game/01_BluePrint/04_UI/HorseGameUI/UI_HorseGame.UI_HorseGame_C" (Game|GetPlayerController 0)))
  (UserInterface|Viewport|AddtoViewport _returnvalue 0)
  (Variables|Default|SetUIHorseGame _returnvalue))

(event Collision|EventActorBeginOverlap
  (params (OtherActor :type Actor%20Object%20Reference)))

(event EventTick
  (params (DeltaSeconds :type Float%20%28single-precision%29)))

(fn ConstructionScript)