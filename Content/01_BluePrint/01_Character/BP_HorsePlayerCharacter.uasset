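; Player horse character for the horse race minigame, steered by yawing with Enhanced Input, with forward movement and jump.
; Tick switches normal, fast and fever states, setting max speed and interpolated camera arm length, narrows turn rate at speed, and feeds finish progress and speed to the HUD.
; High-speed hits play a throttled block montage.
; End events, one playing an ending sequence, flag the save as restart and open L_Mainroom.
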(event Custom|HorsegameEndTriggerSpeedLow
  (Development|SetHiddeninGame (Variables|Character|GetMesh) true false)
  (Variables|Default|SetisEndingSequence true)
  (bind _returnvalue (Sequencer|Player|CreateLevelSequencePlayer "/Game/07_sequence/horsegame/horse_end.horse_end"))
  (Sequencer|Player|Play _returnvalue :!class /Script/MovieScene.MovieSceneSequencePlayer)
  (Utilities|FlowControl|Delay 7.0)
  (bind _returnvalue_2 (SaveGame|LoadGamefromSlot "0"))
  (bind _asbp_save_game (Utilities|Casting|CastToBP_SaveGame _returnvalue_2))
  (Variables|/Game/01_BluePrint/04_UI/MainroomUI/BP_SaveGame.BP_SaveGame_C|SetisRestart _asbp_save_game true)
  (SaveGame|SaveGametoSlot _asbp_save_game (Utilities|String|ToString(Integer) (Variables|/Game/01_BluePrint/04_UI/MainroomUI/BP_SaveGame.BP_SaveGame_C|GetSaveIndex _asbp_save_game)) (Variables|/Game/01_BluePrint/04_UI/MainroomUI/BP_SaveGame.BP_SaveGame_C|GetSaveIndex _asbp_save_game))
  (Game|OpenLevel(byName) "L_Mainroom"))

(event Custom|HorsegameEndTriggerSpeedHigh
  (Utilities|FlowControl|Delay 5.0)
  (bind _returnvalue (SaveGame|LoadGamefromSlot "0"))
  (bind _asbp_save_game (Utilities|Casting|CastToBP_SaveGame _returnvalue))
  (Variables|/Game/01_BluePrint/04_UI/MainroomUI/BP_SaveGame.BP_SaveGame_C|SetisRestart _asbp_save_game true)
  (SaveGame|SaveGametoSlot _asbp_save_game (Utilities|String|ToString(Integer) (Variables|/Game/01_BluePrint/04_UI/MainroomUI/BP_SaveGame.BP_SaveGame_C|GetSaveIndex _asbp_save_game)) (Variables|/Game/01_BluePrint/04_UI/MainroomUI/BP_SaveGame.BP_SaveGame_C|GetSaveIndex _asbp_save_game))
  (Game|OpenLevel(byName) "L_Mainroom"))

(event Input|EnhancedActionEvents|EnhancedInputActionIA_MoveForward
  (params (ActionValue :type Float%20%28double-precision%29) (ElapsedSeconds :type Float%20%28double-precision%29) (TriggeredSeconds :type Float%20%28double-precision%29) (InputAction :type Input%20Action%20Object%20Reference :default "/Game/01_BluePrint/00_Global/00_Input/HorseGame/IA_MoveForward.IA_MoveForward"))
  (CallFunction|MoveForward ActionValue))

(event Input|EnhancedActionEvents|EnhancedInputActionIA_MoveRight
  (params (ActionValue :type Float%20%28double-precision%29) (ElapsedSeconds :type Float%20%28double-precision%29) (TriggeredSeconds :type Float%20%28double-precision%29) (InputAction :type Input%20Action%20Object%20Reference :default "/Game/01_BluePrint/00_Global/00_Input/HorseGame/IA_MoveRight.IA_MoveRight"))
  (CallFunction|MoveLeftRight ActionValue))

(event Input|EnhancedActionEvents|EnhancedInputActionIA_Jump
  (params (ActionValue :type Boolean) (ElapsedSeconds :type Float%20%28double-precision%29) (TriggeredSeconds :type Float%20%28double-precision%29) (InputAction :type Input%20Action%20Object%20Reference :default "/Game/01_BluePrint/00_Global/00_Input/HorseGame/IA_Jump.IA_Jump"))
  (:Started
    (Character|Jump)))

(event EventBeginPlay
  (CallFunction|InitIMContext)
  (CallFunction|CameraArmSetting)
  (bind _returnvalue (Actor|GetActorOfClass "/Game/01_BluePrint/02_Actor/01_Item/HorseGameItem/BP_HorseGameStartLine.BP_HorseGameStartLine_C"))
  (Variables|Default|SetStartLocation (Transformation|GetActorLocation _returnvalue))
  (bind _returnvalue_2 (Actor|GetActorOfClass "/Game/01_BluePrint/02_Actor/01_Item/HorseGameItem/BP_HorseGameFinishLine.BP_HorseGameFinishLine_C"))
  (Variables|Default|SetFinishLocation (Transformation|GetActorLocation _returnvalue_2))
  (Variables|Default|SetStartFinishDistance (Math|Vector|VectorLength (- (Variables|Default|GetFinishLocation) (Variables|Default|GetStartLocation))))
  (bind _asbp_horse_game_hud (Utilities|Casting|CastToBP_HorseGameHud (HUD|GetHUD (Game|GetPlayerController 0))))
  (Variables|Default|SetAs%20BP%20Horse%20Game%20Hud _asbp_horse_game_hud))

(event Collision|EventActorBeginOverlap
  (params (OtherActor :type Actor%20Object%20Reference)))

(event EventTick
  (params (DeltaSeconds :type Float%20%28single-precision%29))
  (Utilities|FlowControl|Sequence
    (:then_0
      (if (Variables|Default|GetisFever)
        (CallFunction|WalkSpeedandCameraArm DeltaSeconds 3e+03 (Variables|Default|GetCurrentArmLength) (Variables|Default|GetFeverArmLength) 1.0)
        (bind _output_get (Variables|Default|SetFeverTime (+ (Variables|Default|GetFeverTime) DeltaSeconds)))
        (if (<= (Variables|Default|GetFeverTimeOut) _output_get)
          (Variables|Default|SetisFever false)
          (Variables|Default|SetFeverTime 0.0))
        (elif (Variables|Default|GetisFast)
          (CallFunction|WalkSpeedandCameraArm DeltaSeconds 1.5e+03 (Variables|Default|GetCurrentArmLength) (Variables|Default|GetFastArmLength) 0.5)
          (else
            (CallFunction|WalkSpeedandCameraArm DeltaSeconds 1e+03 (Variables|Default|GetCurrentArmLength) (Variables|Default|GetDefaultArmLength) 0.5)))))
    (:then_1
      (if (>= (Math|Vector|VectorLength (Variables|/Script/Engine.MovementComponent|GetVelocity (Pawn|GetMovementComponent))) 9.5e+02)
        (Variables|Default|SetisFast true)
        (Variables|/Script/Engine.CharacterMovementComponent|SetRotationRate (Variables|Character|GetCharacterMovement) "0.000000,60.000000,0.000000")
        (else
          (Variables|Default|SetisFast false)
          (Variables|/Script/Engine.CharacterMovementComponent|SetRotationRate (Variables|Character|GetCharacterMovement) "0.000000,120.000000,0.000000"))))
    (:then_2
      (Default|SetFinishLineDistance (Variables|/Game/01_BluePrint/03_FrameWork/BP_HorseGameHud.BP_HorseGameHud_C|GetUIHorseGame (Variables|Default|GetAs%20BP%20Horse%20Game%20Hud)) (- 1.0 (/ (Math|Vector|Distance(Vector) (Transformation|GetActorLocation) (Variables|Default|GetFinishLocation)) (Variables|Default|GetStartFinishDistance)))))
    (:then_3
      (bind _output_get_2 (Variables|Default|SetSpeed (Math|Vector|VectorLength (Transformation|GetVelocity))))
      (Default|SetNowSpeed (Variables|/Game/01_BluePrint/03_FrameWork/BP_HorseGameHud.BP_HorseGameHud_C|GetUIHorseGame (Variables|Default|GetAs%20BP%20Horse%20Game%20Hud)) (/ _output_get_2 3.5e+03) (Utilities|Text|ToText(Integer) (Math|Float|Floor (* (/ _output_get_2 3.5e+03) 3e+02)))))
    (:then_4
      (if (Variables|Default|GetisMontagePlay)
        (bind _output_get_3 (Variables|Default|SetMontagePlayTime (+ (Variables|Default|GetMontagePlayTime) DeltaSeconds)))
        (if (>= _output_get_3 1.0)
          (Variables|Default|SetisMontagePlay false)
          (Variables|Default|SetMontagePlayTime 0.0))))))

(event Collision|EventHit
  (params (MyComp :type Primitive%20Component%20Object%20Reference) (Other :type Actor%20Object%20Reference) (OtherComp :type Primitive%20Component%20Object%20Reference) (bSelfMoved :type Boolean) (HitLocation :type Vector :default "0, 0, 0") (HitNormal :type Vector :default "0, 0, 0") (NormalImpulse :type Vector :default "0, 0, 0") (Hit :type Hit%20Result%20Structure%20%28by%20ref%29))
  (Utilities|FlowControl|Sequence
    (:then_0
      (if (not (Variables|Default|GetisMontagePlay))
        (if (> (Math|Vector|VectorLength (Variables|/Script/Engine.MovementComponent|GetVelocity (Pawn|GetMovementComponent))) 8e+02)
          (Variables|Default|SetisMontagePlay true)
          (Animation|Montage|MontagePlay (Components|SkeletalMesh|GetAnimInstance (Variables|Character|GetMesh)) "/Game/03_Anime/anime_horse/horse_Anime_block.horse_Anime_block" 1.0 "MontageLength" 0.0 false))))))

(fn ConstructionScript)

(fn MoveForward
  (params (ScaleValue :type Float%20%28single-precision%29))
  (Pawn|Input|AddMovementInput (Math|Vector|GetForwardVector (Math|Rotator|MakeRotator 0.0 0.0 (.yaw (Pawn|GetControlRotation :!class /Script/Engine.Pawn)))) ScaleValue false))

(fn MoveLeftRight
  (params (ScaleValue :type Float%20%28single-precision%29))
  (Transformation|AddRelativeRotation (Variables|Collision|GetCapsuleComponent) (Math|Rotator|MakeRotator 0.0 0.0 ScaleValue) false false)
  (Pawn|Input|AddControllerYawInput (* ScaleValue 1.0)))

(fn InitIMContext
  (bind _asbp_player_controller (Utilities|Casting|CastToBP_PlayerController (Pawn|GetController)))
  (Utilities|IsValid _asbp_player_controller
    (:Is%20Valid
      (Input|AddMappingContext (PlayerController|LocalPlayerSubsystems|GetEnhancedInputLocalPlayerSubsystem _asbp_player_controller) "/Game/01_BluePrint/00_Global/00_Input/HorseGame/IM_HorseGameContext.IM_HorseGameContext" 0 "(bIgnoreAllPressedKeysUntilRelease=True,bForceImmediately=False,bNotifyUserSettings=False)")
      (Variables|Default|SetJumpMaxCount 1))))

(fn CameraArmSetting
  (bind _output_get (Variables|Default|SetDefaultArmLength (Variables|/Script/Engine.SpringArmComponent|GetTargetArmLength (Variables|Default|GetSpringArm))))
  (Variables|Default|SetCurrentArmLength _output_get)
  (Variables|Default|SetFastArmLength (* _output_get 2.5))
  (Variables|Default|SetFeverArmLength (* (* _output_get 2.5) 2.0)))

(fn WalkSpeedandCameraArm
  (params (DeltaTime :type Float%20%28double-precision%29) (최대%20걷기%20속도 :type Float%20%28single-precision%29) (Current :type Float%20%28double-precision%29) (Target :type Float%20%28double-precision%29) (InterpSpeed :type Float%20%28double-precision%29))
  (Variables|/Script/Engine.CharacterMovementComponent|SetMaxWalkSpeed (Variables|Character|GetCharacterMovement) 최대%20걷기%20속도)
  (bind _output_get (Variables|Default|SetCurrentArmLength (Math|Interpolation|FInterpTo Current Target DeltaTime InterpSpeed)))
  (Variables|/Script/Engine.SpringArmComponent|SetTargetArmLength (Variables|Default|GetSpringArm) _output_get))