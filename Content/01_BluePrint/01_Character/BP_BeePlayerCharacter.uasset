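; Player bee character that flies by alternating left and right wing inputs, using effectively unlimited jumps.
; Alternating presses flap, triggering a jump plus forward movement input, while repeating the same wing calls SideMove to shift target roll and yaw.
; Tick interpolates control and capsule rotation toward that target and a desired roll, turning slower while falling and zeroing target roll otherwise.
; SideMove's sideways impulse is multiplied by zero, so it only turns.
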(event Input|EnhancedActionEvents|EnhancedInputActionIA_BeeLeftWing
  (params (ActionValue :type Boolean) (ElapsedSeconds :type Float%20%28double-precision%29) (TriggeredSeconds :type Float%20%28double-precision%29) (InputAction :type Input%20Action%20Object%20Reference :default "/Game/01_BluePrint/00_Global/00_Input/BeeGame/IA_BeeLeftWing.IA_BeeLeftWing"))
  (:Started
    (if (Variables|Default|GetisPrevLeft)
      (CallFunction|SideMove (* (Variables|Default|GetPower) -1.0))
      (else
        (Variables|Default|SetisPrevLeft true)
        (CallFunction|Flapping)))))

(event Input|EnhancedActionEvents|EnhancedInputActionIA_BeeRightWing
  (params (ActionValue :type Boolean) (ElapsedSeconds :type Float%20%28double-precision%29) (TriggeredSeconds :type Float%20%28double-precision%29) (InputAction :type Input%20Action%20Object%20Reference :default "/Game/01_BluePrint/00_Global/00_Input/BeeGame/IA_BeeRightWing.IA_BeeRightWing"))
  (:Started
    (if (Variables|Default|GetisPrevLeft)
      (Variables|Default|SetisPrevLeft false)
      (CallFunction|Flapping)
      (else
        (CallFunction|SideMove (* (Variables|Default|GetPower) 1.0))))))

(event EventBeginPlay
  (bind _returnvalue (Pawn|GetControlRotation :!class /Script/Engine.Pawn))
  (bind _asbp_player_controller (Utilities|Casting|CastToBP_PlayerController (Pawn|GetController)))
  (Utilities|IsValid _asbp_player_controller
    (:Is%20Valid
      (Input|AddMappingContext (PlayerController|LocalPlayerSubsystems|GetEnhancedInputLocalPlayerSubsystem _asbp_player_controller) "/Game/01_BluePrint/00_Global/00_Input/BeeGame/IM_BeeGameContext.IM_BeeGameContext" 0 "(bIgnoreAllPressedKeysUntilRelease=True,bForceImmediately=False,bNotifyUserSettings=False)")
      (Variables|Default|SetJumpMaxCount 2147483647)
      (Variables|Default|SetTargetRotation _returnvalue)
      (Variables|Default|SetCurrentRotation _returnvalue))))

(event Collision|EventActorBeginOverlap
  (params (OtherActor :type Actor%20Object%20Reference)))

(event EventTick
  (params (DeltaSeconds :type Float%20%28single-precision%29))
  (Utilities|FlowControl|Sequence
    (:then_0
      (Pawn|SetControlRotation (Pawn|GetController) (Math|Interpolation|RInterpTo (Variables|Default|GetCurrentRotation) (Math|Rotator|MakeRotator (Variables|Default|GetdisireRoll) (.pitch (Variables|Default|GetCurrentRotation)) (.yaw (Variables|Default|GetCurrentRotation))) DeltaSeconds 0.3))
      (bind _output_get (Variables|Default|SetCurrentRotation (Math|Interpolation|RInterpTo (Variables|Default|GetCurrentRotation) (Math|Rotator|MakeRotator (Variables|Default|GetdisireRoll) (.pitch (Variables|Default|GetCurrentRotation)) (.yaw (Variables|Default|GetCurrentRotation))) DeltaSeconds 0.3)))
      (Transformation|SetWorldRotation (Variables|Collision|GetCapsuleComponent) _output_get false false))
    (:then_1
      (if (Utilities|Operators|NotEqual(!=) (Variables|Default|GetCurrentRotation) (Variables|Default|GetTargetRotation) 0.0)
        (Pawn|SetControlRotation (Pawn|GetController) (Math|Interpolation|RInterpTo (Variables|Default|GetCurrentRotation) (Variables|Default|GetTargetRotation) DeltaSeconds (Variables|Default|GetInterp%20Speed)))
        (bind _output_get_2 (Variables|Default|SetCurrentRotation (Math|Interpolation|RInterpTo (Variables|Default|GetCurrentRotation) (Variables|Default|GetTargetRotation) DeltaSeconds (Variables|Default|GetInterp%20Speed))))
        (Transformation|SetWorldRotation (Variables|Collision|GetCapsuleComponent) _output_get_2 false false)))
    (:then_2
      (if (AI|Components|NavMovement|IsFalling (Variables|Character|GetCharacterMovement))
        (Variables|Default|SetInterp%20Speed 0.3)
        (else
          (Variables|Default|SetInterp%20Speed 1.0)
          (Variables|Default|SetTargetRotation (Math|Rotator|MakeRotator 0.0 (.pitch (Variables|Default|GetCurrentRotation)) (.yaw (Variables|Default|GetCurrentRotation)))))))))

(fn ConstructionScript)

(fn Flapping
  (Character|Jump)
  (Pawn|Input|AddMovementInput (Math|Vector|GetForwardVector (Pawn|GetControlRotation :!class /Script/Engine.Pawn)) 1e+03 false))

(fn SideMove
  (params (Power :type Float%20%28double-precision%29))
  (bind _currentrotation (Variables|Default|GetCurrentRotation))
  (Physics|AddImpulse (Variables|Character|GetCharacterMovement) (* (Math|Vector|GetRightVector (Math|Rotator|MakeRotator 0.0 0.0 (.yaw (Pawn|GetControlRotation :!class /Script/Engine.Pawn)))) "") false)
  (Variables|Default|SetTargetRotation (Math|Rotator|MakeRotator (+ (.roll _currentrotation) (* Power 5e+01)) (.pitch _currentrotation) (+ (.yaw _currentrotation) (* Power 5e+01)))))