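; Player character for the escape game, with Enhanced Input movement, camera zoom, fall recovery and item interaction.
; Jump also attempts a mantle, using sphere traces to find the ledge and motion warping to drive the climb montage.
; Tagged pickups use a stacking slot inventory that tries the equipped, droppable backpack first and refreshes by recreating its widget.
; Hotkeys consume pill, leaf or teleporter items, with Tick timing pill duration and delayed teleport to SaveLocation.
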(event Custom|RefreshWidget
  ;[0 0 0] Inventory Key
  (Utilities|FlowControl|Sequence
    (:then_0
      (Variables|/Script/Engine.PlayerController|SetbShowMouseCursor (Widget|GetOwningPlayer (Variables|Default|GetUI_Inventory)) false)
      (Input|SetInputModeGameOnly (Widget|GetOwningPlayer (Variables|Default|GetUI_Inventory)) false)
      (Widget|RemovefromParent (Variables|Default|GetUI_Inventory))
      (Variables|Default|SetisViewInventory false))
    (:then_1
      (bind _returnvalue (UserInterface|CreateWidget "/Game/01_BluePrint/04_UI/EscapeGameUI/UI_Inventory.UI_Inventory_C"))
      (bind _output_get (Variables|Default|SetUI_Inventory _returnvalue))
      (UserInterface|Viewport|AddtoViewport _output_get 0)
      (Variables|/Script/Engine.PlayerController|SetbShowMouseCursor (Widget|GetOwningPlayer (Variables|Default|GetUI_Inventory)) true)
      (Input|SetInputModeGameandUI (Widget|GetOwningPlayer (Variables|Default|GetUI_Inventory)) (Variables|Default|GetUI_Inventory) "DoNotLock" true false)
      (Variables|Default|SetisViewInventory true))))

(event Input|EnhancedActionEvents|EnhancedInputActionIA_MoveForward
  (params (ActionValue :type Float%20%28double-precision%29) (ElapsedSeconds :type Float%20%28double-precision%29) (TriggeredSeconds :type Float%20%28double-precision%29) (InputAction :type Input%20Action%20Object%20Reference :default "/Game/01_BluePrint/00_Global/00_Input/HorseGame/IA_MoveForward.IA_MoveForward"))
  ;[0 0 0] MoveCharacater
  (CallFunction|MoveForward ActionValue))

(event Input|EnhancedActionEvents|EnhancedInputActionIA_MoveRight
  (params (ActionValue :type Float%20%28double-precision%29) (ElapsedSeconds :type Float%20%28double-precision%29) (TriggeredSeconds :type Float%20%28double-precision%29) (InputAction :type Input%20Action%20Object%20Reference :default "/Game/01_BluePrint/00_Global/00_Input/HorseGame/IA_MoveRight.IA_MoveRight"))
  ;[0 0 0] MoveCharacater
  (CallFunction|MoveLeftRight ActionValue))

(event Input|EnhancedActionEvents|EnhancedInputActionIA_UseItem3
  (params (ActionValue :type Boolean) (ElapsedSeconds :type Float%20%28double-precision%29) (TriggeredSeconds :type Float%20%28double-precision%29) (InputAction :type Input%20Action%20Object%20Reference :default "/Game/01_BluePrint/00_Global/00_Input/EscapeGame/Test/IA_UseItem3.IA_UseItem3"))
  (:Started
    (CallFunction|UseItem 2)))

(event Input|EnhancedActionEvents|EnhancedInputActionIA_Jump
  (params (ActionValue :type Boolean) (ElapsedSeconds :type Float%20%28double-precision%29) (TriggeredSeconds :type Float%20%28double-precision%29) (InputAction :type Input%20Action%20Object%20Reference :default "/Game/01_BluePrint/00_Global/00_Input/HorseGame/IA_Jump.IA_Jump"))
  ;[0 0 0] MoveCharacater
  (:Started
    (Utilities|FlowControl|Sequence
      (:then_0
        (if (not (AI|Components|NavMovement|IsFalling (Variables|Character|GetCharacterMovement)))
          (if (not (Variables|Default|Getis_mantle))
            (Character|Jump)
            (Animation|Montage|PlayMontage (Variables|Character|GetMesh) "/Game/03_Anime/anime_bean/beancharacter_jumpM1.beancharacter_jumpM1"))))
      (:then_1
        ;[1 1 1] mantling
        (bind (_motion1 _motion2) (CallFunction|MantleTrace 1.2e+02 2e+02 0.5 "ForDuration"))
        (if (Variables|Default|Getcanmantle)
          (if (not (Variables|Default|Getis_mantle))
            (Variables|Default|Setis_mantle true)
            (Utilities|Mantle _motion1 _motion2 -1e+02 3e+01 1.92)
            (Variables|Default|Setis_mantle false)))))))

(event Input|EnhancedActionEvents|EnhancedInputActionIA_Interaction
  (params (ActionValue :type Boolean) (ElapsedSeconds :type Float%20%28double-precision%29) (TriggeredSeconds :type Float%20%28double-precision%29) (InputAction :type Input%20Action%20Object%20Reference :default "/Game/01_BluePrint/00_Global/00_Input/EscapeGame/Test/IA_Interaction.IA_Interaction"))
  (bind _capsulecomponent (Variables|Collision|GetCapsuleComponent))
  (bind _returnvalue (Transformation|GetWorldLocation _capsulecomponent))
  ;[0 0 0] ItemInteraction
  (:Completed
    (bind (_outhit _returnvalue_2) (Collision|SphereTraceByChannel _returnvalue _returnvalue 8e+01 "TraceTypeQuery1" false 0 "ForDuration"))
    (if _returnvalue_2
      (if (Actor|ActorHasTag (.HitActor (Collision|BreakHitResult _outhit)) "PickUp")
        (Class|BPIPickUpInteraction|PickUpInteraction(Message) (.HitActor (Collision|BreakHitResult _outhit)) self)
        (if (Variables|Default|GetisViewInventory)
          (CallFunction|RefreshWidget))))))

(event Input|EnhancedActionEvents|EnhancedInputActionIA_Inventory
  (params (ActionValue :type Boolean) (ElapsedSeconds :type Float%20%28double-precision%29) (TriggeredSeconds :type Float%20%28double-precision%29) (InputAction :type Input%20Action%20Object%20Reference :default "/Game/01_BluePrint/00_Global/00_Input/EscapeGame/Test/IA_Inventory.IA_Inventory"))
  ;[0 0 0] Inventory Key
  (:Started
    (Utilities|FlowControl|FlipFlop
      (:A
        (bind _returnvalue (UserInterface|CreateWidget "/Game/01_BluePrint/04_UI/EscapeGameUI/UI_Inventory.UI_Inventory_C"))
        (bind _output_get (Variables|Default|SetUI_Inventory _returnvalue))
        (UserInterface|Viewport|AddtoViewport _output_get 0)
        (Variables|/Script/Engine.PlayerController|SetbShowMouseCursor (Widget|GetOwningPlayer (Variables|Default|GetUI_Inventory)) true)
        (Input|SetInputModeGameandUI (Widget|GetOwningPlayer (Variables|Default|GetUI_Inventory)) (Variables|Default|GetUI_Inventory) "DoNotLock" true false)
        (Variables|Default|SetisViewInventory true))
      (:B
        (Variables|/Script/Engine.PlayerController|SetbShowMouseCursor (Widget|GetOwningPlayer (Variables|Default|GetUI_Inventory)) false)
        (Input|SetInputModeGameOnly (Widget|GetOwningPlayer (Variables|Default|GetUI_Inventory)) false)
        (Widget|RemovefromParent (Variables|Default|GetUI_Inventory))
        (Variables|Default|SetisViewInventory false)))))

(event Input|EnhancedActionEvents|EnhancedInputActionIA_Backpack
  (params (ActionValue :type Boolean) (ElapsedSeconds :type Float%20%28double-precision%29) (TriggeredSeconds :type Float%20%28double-precision%29) (InputAction :type Input%20Action%20Object%20Reference :default "/Game/01_BluePrint/00_Global/00_Input/EscapeGame/Test/IA_Backpack.IA_Backpack"))
  (bind _equipbackpack (Variables|Default|GetEquipBackpack))
  (bind _capsulecomponent (Variables|Collision|GetCapsuleComponent))
  ;[0 0 0] Backpack Drop
  (:Started
    (Utilities|IsValid _equipbackpack
      (:Is%20Valid
        (Game|SpawnActorfromClass "/Game/06_Inventory/Backpack_Master.Backpack_Master_C" (Math|Transform|MakeTransform (+ (Transformation|GetWorldLocation _capsulecomponent) (* (Math|Vector|GetForwardVector _capsulecomponent) 200)) "0, 0, 0" "1.000000,1.000000,1.000000") "Undefined" "MultiplyWithRoot" _equipbackpack (Variables|/Game/06_Inventory/Backpack_Master.Backpack_Master_C|GetBackpackSlot _equipbackpack) (Utilities|Struct|MakeS_Backpacks (Utilities|Struct|BreakS_Backpacks (Variables|/Game/06_Inventory/Backpack_Master.Backpack_Master_C|GetBackpackType (Variables|Default|GetEquipBackpack)))) 0)
        (Actor|DestroyActor _equipbackpack)
        (if (Variables|Default|GetisViewInventory)
          (CallFunction|RefreshWidget))))))

(event Input|EnhancedActionEvents|EnhancedInputActionIA_MouseXY
  (params (ActionValue :type Vector%202D%20Structure) (ElapsedSeconds :type Float%20%28double-precision%29) (TriggeredSeconds :type Float%20%28double-precision%29) (InputAction :type Input%20Action%20Object%20Reference :default "/Game/01_BluePrint/00_Global/00_Input/EscapeGame/Test/IA_MouseXY.IA_MouseXY"))
  ;[1 1 1] Camera
  (CallFunction|MouseCamera (.x ActionValue) (.y ActionValue)))

(event Input|EnhancedActionEvents|EnhancedInputActionIA_MouseWheel
  (params (ActionValue :type Float%20%28double-precision%29) (ElapsedSeconds :type Float%20%28double-precision%29) (TriggeredSeconds :type Float%20%28double-precision%29) (InputAction :type Input%20Action%20Object%20Reference :default "/Game/01_BluePrint/00_Global/00_Input/EscapeGame/Test/IA_MouseWheel.IA_MouseWheel"))
  ;[1 1 1] Camera
  (CallFunction|CameraArmSetting ActionValue))

(event Input|EnhancedActionEvents|EnhancedInputActionIA_UseItem1
  (params (ActionValue :type Boolean) (ElapsedSeconds :type Float%20%28double-precision%29) (TriggeredSeconds :type Float%20%28double-precision%29) (InputAction :type Input%20Action%20Object%20Reference :default "/Game/01_BluePrint/00_Global/00_Input/EscapeGame/Test/IA_UseItem1.IA_UseItem1"))
  (:Started
    (CallFunction|UseItem)))

(event Input|EnhancedActionEvents|EnhancedInputActionIA_UseItem2
  (params (ActionValue :type Boolean) (ElapsedSeconds :type Float%20%28double-precision%29) (TriggeredSeconds :type Float%20%28double-precision%29) (InputAction :type Input%20Action%20Object%20Reference :default "/Game/01_BluePrint/00_Global/00_Input/EscapeGame/Test/IA_UseItem2.IA_UseItem2"))
  (:Started
    (CallFunction|UseItem 1)))

(event EventBeginPlay
  (CallFunction|InitIMContext))

(event Collision|EventActorBeginOverlap
  (params (OtherActor :type Actor%20Object%20Reference)))

(event EventTick
  (params (DeltaSeconds :type Float%20%28single-precision%29))
  (Utilities|FlowControl|Sequence
    (:then_0
      (if (Variables|Default|GetisEatPill)
        (bind _output_get (Variables|Default|SetPillDuration (+ (Variables|Default|GetPillDuration) DeltaSeconds)))
        (if (>= _output_get 5.0)
          (Variables|Default|SetisEatPill false)
          (Variables|Default|SetPillDuration 0.0))))
    (:then_1
      (if (Variables|Default|GetisTeleport)
        (bind _output_get_2 (Variables|Default|SetTeleportDuration%20 (+ (Variables|Default|GetTeleportDuration%20) DeltaSeconds)))
        (if (>= _output_get_2 0.5)
          (Components|Activation|Activate (Variables|Default|GetNiagara) false)
          (Transformation|SetActorLocation (Variables|Default|GetsaveLocation) false true)
          (Variables|Default|SetisTeleport false)
          (Variables|Default|SetTeleportDuration%20 0.0))))
    (:then_2
      (if (<= (.z (Transformation|GetWorldLocation (Variables|Character|GetMesh))) -5e+02)
        (Transformation|SetActorLocation "3650.000000,5350.000000,192.000000" false true)))))

(event Input|KeyboardEvents|NumPadZero
  (params (Key :type Key%20Structure :default "None"))
  ;[0 0 0] Debug_Inventory
  (:Pressed
    (for _array_element (Variables|Default|GetPlayerSlot)
      (Development|PrintString (Utilities|String|ToString(Name) (.RowName (Utilities|Struct|BreakDataTableRowHandle (.Item (Utilities|Struct|BreakS_Slots _array_element))))))
      (Development|PrintString (Utilities|String|ToString(Integer) (.Amount (Utilities|Struct|BreakS_Slots _array_element)))))))

(fn ConstructionScript)

(fn MoveForward
  (params (ScaleValue :type Float%20%28single-precision%29))
  (Pawn|Input|AddMovementInput (Math|Vector|GetForwardVector (Math|Rotator|MakeRotator 0.0 0.0 (.yaw (Pawn|GetControlRotation :!class /Script/Engine.Pawn)))) ScaleValue false))

(fn MoveLeftRight
  (params (ScaleValue :type Float%20%28single-precision%29))
  ;[1 1 1] 옆으로움직이기
  (Pawn|Input|AddMovementInput (Math|Vector|GetRightVector (Math|Rotator|MakeRotator 0.0 0.0 (.yaw (Pawn|GetControlRotation :!class /Script/Engine.Pawn)))) ScaleValue false))

(fn InitIMContext
  (bind _asbp_player_controller (Utilities|Casting|CastToBP_PlayerController (Pawn|GetController)))
  (Utilities|IsValid _asbp_player_controller
    (:Is%20Valid
      (Input|AddMappingContext (PlayerController|LocalPlayerSubsystems|GetEnhancedInputLocalPlayerSubsystem _asbp_player_controller) "/Game/01_BluePrint/00_Global/00_Input/EscapeGame/Test/IM_EscapeGameContext.IM_EscapeGameContext" 0 "(bIgnoreAllPressedKeysUntilRelease=True,bForceImmediately=False,bNotifyUserSettings=False)")
      (Variables|Default|SetJumpMaxCount 1))))

(fn AddItem
  (params (PickUpItem :type S%20Slots%20Structure) (Source :type String))
  (bind _equipbackpack (Variables|Default|GetEquipBackpack))
  (LocalVariables|SetLocalPickUpItem PickUpItem)
  (switch string Source
    (:Ground
      (Utilities|IsValid _equipbackpack
        (:Is%20Valid
          (bind _success (Default|AddItem _equipbackpack (LocalVariables|GetLocalPickUpItem)))
          (if _success
            (return true)
            (else
              _)))
        (:Is%20Not%20Valid
          _))
      (bind (_success_2 _itemindex) (CallFunction|FindStack (LocalVariables|GetLocalPickUpItem)))
      (bind _output_get (LocalVariables|SetLocalPlayerItemIndex _itemindex))
      (if _success_2
        (bind _success_3 (CallFunction|WhetherCanStack (LocalVariables|GetLocalPickUpItem) _output_get))
        (if _success_3
          (bind _success_4 (CallFunction|IncreaseItemAmounttoPlayerSlot (LocalVariables|GetLocalPlayerItemIndex)))
          (return _success_4)
          (else
            _)))
      (bind (_success_5 _index) (CallFunction|FindEmpty))
      (if _success_5
        (bind _success_6 (CallFunction|AddItemtoPlayerSlot (LocalVariables|GetLocalPickUpItem) _index))
        (return _success_6)
        (else
          (return false))))))

(fn FindEmpty
  (bind (_array_element _array_index) (Utilities|Array|ForEachLoopwithBreak (Variables|Default|GetPlayerSlot) :!label _label)
    (:LoopBody
      (if (== (.RowName (Utilities|Struct|BreakDataTableRowHandle (.Item (Utilities|Struct|BreakS_Slots _array_element)))) (Variables|Default|GetEmpty))
        (LocalVariables|SetLocalFound true)
        (LocalVariables|SetLocalIndex _array_index)
        (goto _label Break)
        (else
          (LocalVariables|SetLocalFound false))))
    (:Completed
      (return (LocalVariables|GetLocalFound) (LocalVariables|GetLocalIndex)))))

(fn IncreaseItemAmounttoPlayerSlot
  (params (Index :type Integer))
  (bind _playerslot (Variables|Default|GetPlayerSlot))
  (bind _output (Utilities|Array|Get(acopy) _playerslot Index))
  (Utilities|Array|SetArrayElem (Variables|Default|GetPlayerSlot) Index (Utilities|Struct|MakeS_Slots (.item _output) (+ (.amount _output) 1)))
  (return true))

(fn FindStack
  (params (FindStack :type S%20Slots%20Structure))
  ;[0 0 0] 픽업아이템이 플레이어 인벤토리에 존재하는 물건인지 확인
  (bind (_array_element _array_index) (Utilities|Array|ForEachLoopwithBreak (Variables|Default|GetPlayerSlot) :!label _label)
    (:LoopBody
      (if (== (.RowName (Utilities|Struct|BreakDataTableRowHandle (.Item (Utilities|Struct|BreakS_Slots _array_element)))) (.RowName (Utilities|Struct|BreakDataTableRowHandle (.Item (Utilities|Struct|BreakS_Slots FindStack)))))
        (LocalVariables|SetLocalFound true)
        (LocalVariables|SetLocalIndex _array_index)
        (LocalVariables|SetLocalAmount (.Amount (Utilities|Struct|BreakS_Slots _array_element)))
        (goto _label Break)))
    (:Completed
      (return (LocalVariables|GetLocalFound) (LocalVariables|GetLocalIndex) (LocalVariables|GetLocalAmount)))))

(fn WhetherCanStack
  (params (GetItem :type S%20Slots%20Structure) (PlayerItemIndex :type Integer))
  (bind _playerslot (Variables|Default|GetPlayerSlot))
  (bind _output (Utilities|Array|Get(acopy) _playerslot PlayerItemIndex))
  (bind (_datatable _rowname) (Utilities|Struct|BreakDataTableRowHandle (.item _output)))
  (bind _returnvalue (Utilities|GetDataTableRow _datatable _rowname)
    (:then
      (if (.CanStack (Utilities|Struct|BreakS_Inventory _returnvalue))
        (Development|PrintString "Can Stack")
        (return true)
        (else
          (Development|PrintString "Can Not Stack")
          (return false))))
    (:RowNotFound
      (Development|PrintString "Row Not Found")
      (return false))))

(fn AddItemtoPlayerSlot
  (params (PickUpItem :type S%20Slots%20Structure) (InventoryIndex :type Integer))
  (Utilities|Array|SetArrayElem (Variables|Default|GetPlayerSlot) InventoryIndex (Utilities|Struct|MakeS_Slots (.Item (Utilities|Struct|BreakS_Slots PickUpItem)) 1))
  (return true))

(fn RemoveItem
  (params (RemoveItem :type S%20Slots%20Structure))
  (bind (_item _amount) (Utilities|Struct|BreakS_Slots RemoveItem))
  (bind _playerslot (Variables|Default|GetPlayerSlot))
  (bind (_success _itemindex _itemamount) (CallFunction|FindStack RemoveItem))
  (LocalVariables|SetLocalItemIndex _itemindex)
  (LocalVariables|SetLocalItemAmount _itemamount)
  (if _success
    (if (<= (- _itemamount _amount) 0)
      (Utilities|Array|SetArrayElem _playerslot (LocalVariables|GetLocalItemIndex) (Utilities|Struct|MakeS_Slots (Utilities|Struct|MakeDataTableRowHandle "/Game/06_Inventory/ItemDataTable.ItemDataTable" "Empty") 0))
      (else
        (Utilities|Array|SetArrayElem _playerslot (LocalVariables|GetLocalItemIndex) (Utilities|Struct|MakeS_Slots _item (- _itemamount _amount)))))
    (return true)
    (else
      (return false))))

(fn RemoveItematIndex
  (params (Index :type Integer) (AmountRemove :type Integer))
  (bind _playerslot (Variables|Default|GetPlayerSlot))
  (bind _output_get (LocalVariables|SetLocalRemoveIndex Index))
  (if (<= (Utilities|Operators|Subtract (.amount (Utilities|Array|Get(acopy) (Variables|Default|GetPlayerSlot) _output_get)) AmountRemove) 0)
    (Utilities|Array|SetArrayElem _playerslot (LocalVariables|GetLocalRemoveIndex) (Utilities|Struct|MakeS_Slots (Utilities|Struct|MakeDataTableRowHandle "/Game/06_Inventory/ItemDataTable.ItemDataTable" "Empty") 0))
    (else
      (Utilities|Array|SetArrayElem _playerslot (LocalVariables|GetLocalRemoveIndex) (Utilities|Struct|MakeS_Slots (.item (Utilities|Array|Get(acopy) (Variables|Default|GetPlayerSlot) _output_get)) (Utilities|Operators|Subtract (.amount (Utilities|Array|Get(acopy) (Variables|Default|GetPlayerSlot) _output_get)) AmountRemove)))))
  (return true))

(fn MantleTrace
  (params (initial_trace_length :type Float%20%28double-precision%29) (Z_offset :type Float%20%28double-precision%29) (falling_height :type Float%20%28double-precision%29) (Debugtrace :type EDrawDebugTrace%20Enum :default "None"))
  (bind _returnvalue (Transformation|GetActorLocation))
  (bind _returnvalue_2 (Transformation|GetActorForwardVector))
  (bind _returnvalue_3 (* initial_trace_length _returnvalue_2))
  (bind _returnvalue_4 (+ _returnvalue _returnvalue_3))
  (bind _returnvalue_5 (+ (.z _returnvalue_4) 3e+01))
  (bind _returnvalue_6 (Math|Vector|MakeVector (.x _returnvalue_4) (.y _returnvalue_4) _returnvalue_5))
  (Variables|Default|Setcanmantle false)
  (bind (_outhit _returnvalue_7) (Collision|SphereTraceByChannel _returnvalue_6 _returnvalue_6 8e+01 "TraceTypeQuery1" false 0 Debugtrace))
  (if _returnvalue_7
    (bind (_outhit_2 _returnvalue_8) (Collision|SphereTraceByChannel (+ (.Location (Collision|BreakHitResult _outhit)) (Math|Vector|MakeVector 0.0 0.0 (* Z_offset (Math|Float|SelectFloat falling_height 1.0 (AI|Components|NavMovement|IsFalling (Variables|Character|GetCharacterMovement)))))) (.Location (Collision|BreakHitResult _outhit)) 1e+01 "TraceTypeQuery1" false 0 Debugtrace))
    (if _returnvalue_8
      (LocalVariables|Setmotionposi1 (+ (.ImpactPoint (Collision|BreakHitResult _outhit_2)) (* (Transformation|GetActorForwardVector) -5e+01)))
      (bind _output_get (LocalVariables|Setmotionposi2 (+ (* (Transformation|GetActorForwardVector) 1.2e+02) (.ImpactPoint (Collision|BreakHitResult _outhit_2)))))
      (Variables|Default|Setcanmantle true)
      (bind _returnvalue_9 (Collision|SphereTraceByChannel (+ _output_get "0.000000,0.000000,20.000000") (+ _output_get "0.000000,0.000000,20.000000") 1e+01 "TraceTypeQuery1" false 0 Debugtrace))
      (if _returnvalue_9
        (Variables|Default|Setcanmantle false)
        (else
          (LocalVariables|Setmotionposi2 (+ (.ImpactPoint (Collision|BreakHitResult _outhit_2)) (* (Transformation|GetActorForwardVector) 5e+01)))))
      (if (or (Utilities|Operators|EqualEqual :A (LocalVariables|Getmotionposi1)) (Utilities|Operators|EqualEqual :A (LocalVariables|Getmotionposi2)))
        (Variables|Default|Setcanmantle false :!label _label)
        (else
          (bind _returnvalue_10 (Collision|SphereTraceByChannel (Math|Vector|MakeVector (.x (LocalVariables|Getmotionposi1)) (.y (LocalVariables|Getmotionposi1)) (.Z (Math|Vector|BreakVector (+ (LocalVariables|Getmotionposi2) "0.000000,0.000000,50.000000")))) (+ (LocalVariables|Getmotionposi2) "0.000000,0.000000,50.000000") 2e+01 "TraceTypeQuery1" false 0 Debugtrace))
          (if _returnvalue_10
            (goto _label)
            (else
              _))))
      (return (LocalVariables|Getmotionposi1) (LocalVariables|Getmotionposi2)))
    (else
      (Variables|Default|Setcanmantle false))))

(fn Mantletset
  (params (location1 :type Vector) (location2 :type Vector) (zoffsethandle :type Float%20%28double-precision%29) (zoffsetlanding :type Float%20%28double-precision%29) (montagelength :type Float%20%28double-precision%29))
  (Collision|SetActorEnableCollision false)
  (Pawn|Components|CharacterMovement|SetMovementMode (Variables|Character|GetCharacterMovement) "MOVE_Flying" 0)
  (Class|MotionWarpingComponent|AddorUpdateWarpTarget (Variables|Default|GetMotionWarping) (Utilities|Struct|MakeMotionWarpingTarget "loca1" (+ location1 (Math|Vector|MakeVector 0.0 0.0 (+ zoffsethandle 1e+03))) (Transformation|GetActorRotation)))
  (Class|MotionWarpingComponent|AddorUpdateWarpTarget (Variables|Default|GetMotionWarping) (Utilities|Struct|MakeMotionWarpingTarget "loca2" (+ location2 (Math|Vector|MakeVector 0.0 0.0 (+ zoffsetlanding 2e+01))) (Transformation|GetActorRotation)))
  (Animation|PlayAnimMontage "/Game/03_Anime/anime_bean/beancharacterclimb1_Montage.beancharacterclimb1_Montage" 1.0 "None")
  (Collision|SetActorEnableCollision true)
  (Pawn|Components|CharacterMovement|SetMovementMode (Variables|Character|GetCharacterMovement) "MOVE_Falling" 0))

(fn MouseCamera
  (params (Val :type Float%20%28single-precision%29) (Val2 :type Float%20%28single-precision%29))
  ;[1 1 1] 마우스로 카메라시선처리
  (Pawn|Input|AddControllerYawInput Val)
  (Pawn|Input|AddControllerPitchInput Val2))

(fn CameraArmSetting
  (params (A :type Float%20%28double-precision%29))
  ;[1 1 1] 카메라 스프링 암 조작
  (Variables|/Script/Engine.SpringArmComponent|SetTargetArmLength (Variables|Default|GetSpringArm) (Math|Float|Clamp(Float) (+ (Variables|/Script/Engine.SpringArmComponent|GetTargetArmLength (Variables|Default|GetSpringArm)) (* A (Variables|Default|GetSpeedWheel))) 1e+02 1.5e+03)))

(fn UseItem
  (params (Index :type Integer))
  (bind _capsulecomponent (Variables|Collision|GetCapsuleComponent))
  (bind _playerslot (Variables|Default|GetPlayerSlot))
  (bind _returnvalue (Math|Vector|GetForwardVector _capsulecomponent))
  (bind _returnvalue_2 (Transformation|GetWorldLocation _capsulecomponent))
  (bind _output (Utilities|Array|Get(acopy) _playerslot Index))
  (bind (_item _amount) (Utilities|Struct|BreakS_Slots _output))
  (bind _returnvalue_3 (* _returnvalue 5e+02))
  (bind _returnvalue_4 (+ _returnvalue_3 _returnvalue_2))
  (if (>= _amount 1)
    (switch name (.RowName (Utilities|Struct|BreakDataTableRowHandle _item))
      (:GreenPill
        (CallFunction|RemoveItematIndex Index 1)
        (Variables|Default|SetisEatPill true)
        (if (Variables|Default|GetisViewInventory)
          (CallFunction|RefreshWidget)))
      (:Leaf
        (CallFunction|RemoveItematIndex Index 1)
        (Game|SpawnActorfromClass "/Game/01_BluePrint/02_Actor/00_Monster/BP_ItemSmallLeaf.BP_ItemSmallLeaf_C" (Math|Transform|MakeTransform (Math|Vector|MakeVector (.x _returnvalue_4) (.y _returnvalue_4) (+ (.z _returnvalue_4) 5e+01)) (Variables|/Script/Engine.SceneComponent|GetRelativeRotation _capsulecomponent) "1.000000,1.000000,1.000000") "Undefined" "MultiplyWithRoot" 0 0)
        (if (Variables|Default|GetisViewInventory)
          (CallFunction|RefreshWidget)))
      (:Teleporter
        (CallFunction|RemoveItematIndex Index 1)
        (Components|SkeletalMesh|SetSkeletalMeshAsset (Variables|Character|GetMesh) "/Game/02_Assets/A_Character/C_beancharacter/beancharacterteleport.beancharacterteleport")
        (Animation|PlayAnimMontage "/Game/03_Anime/anime_bean/beancharacter_teleport_Montage.beancharacter_teleport_Montage" 1.0 "None")
        (Components|SkeletalMesh|SetSkeletalMeshAsset (Variables|Character|GetMesh) "/Game/02_Assets/A_Character/C_beancharacter/Beancharacter.Beancharacter")
        (Variables|Default|SetisTeleport true)
        (if (Variables|Default|GetisViewInventory)
          (CallFunction|RefreshWidget))))))