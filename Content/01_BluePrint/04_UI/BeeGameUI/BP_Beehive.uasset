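; BP_Beehive is the goal actor of the bee game, with a widget marker showing the player's distance to the hive.
; While the marker is enabled, Tick updates the UI_Beehive text in meters, caching the widget reference on first use.
; Sphere overlap hides the marker, plays the Bee_clear sequence, then after a delay flags IsRestart in the save game and opens L_Mainroom.
; It loads slot "0" but saves to the slot named by SaveIndex.
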(event OnComponentBeginOverlap(Sphere)
  (params (OverlappedComponent :type Primitive%20Component%20Object%20Reference) (OtherActor :type Actor%20Object%20Reference) (OtherComp :type Primitive%20Component%20Object%20Reference) (OtherBodyIndex :type Integer) (bFromSweep :type Boolean) (SweepResult :type Hit%20Result%20Structure%20%28by%20ref%29))
  (Rendering|SetVisibility (Variables|Default|GetWidget) false false)
  (bind _returnvalue (Sequencer|Player|CreateLevelSequencePlayer "/Game/07_sequence/beegame/bee_clear.bee_clear"))
  (Sequencer|Player|Play _returnvalue :!class /Script/MovieScene.MovieSceneSequencePlayer)
  (Utilities|FlowControl|Delay 5.2)
  (bind _returnvalue_2 (SaveGame|LoadGamefromSlot "0"))
  (bind _asbp_save_game (Utilities|Casting|CastToBP_SaveGame _returnvalue_2))
  (Variables|/Game/01_BluePrint/04_UI/MainroomUI/BP_SaveGame.BP_SaveGame_C|SetisRestart _asbp_save_game true)
  (SaveGame|SaveGametoSlot _asbp_save_game (Utilities|String|ToString(Integer) (Variables|/Game/01_BluePrint/04_UI/MainroomUI/BP_SaveGame.BP_SaveGame_C|GetSaveIndex _asbp_save_game)) (Variables|/Game/01_BluePrint/04_UI/MainroomUI/BP_SaveGame.BP_SaveGame_C|GetSaveIndex _asbp_save_game))
  (Game|OpenLevel(byName) "L_Mainroom"))

(event EventBeginPlay
  (CallFunction|ToggleObjectiveMarker (Variables|Default|GetWidget) (Variables|Default|GetMarkerEnabled)))

(event Collision|EventActorBeginOverlap
  (params (OtherActor :type Actor%20Object%20Reference)))

(event EventTick
  (params (DeltaSeconds :type Float%20%28single-precision%29))
  (if (Variables|Default|GetMarkerEnabled)
    (CallFunction|UpdateDistance)))

(fn ConstructionScript)

(fn UpdateDistance
  (bind _as_ui_beehive (Variables|Default|GetAs%20UI%20Beehive)
    (:then
      _)
    (:else
      (bind _asui_beehive (Utilities|Casting|CastToUI_Beehive (UserInterface|GetUserWidgetObject (Variables|Default|GetWidget))))
      (Variables|Default|SetAs%20UI%20Beehive _asui_beehive)))
  (Default|HiveUpdateText _as_ui_beehive (Utilities|Text|ToText(String) (Utilities|String|Append (Utilities|String|ToString(Integer) (Math|Float|Round (/ (Math|Vector|Distance(Vector) (Transformation|GetActorLocation (Game|GetPlayerCharacter 0)) (Transformation|GetActorLocation)) 1e+02))) "m"))))

(fn ToggleObjectiveMarker
  (params (self2 :type Scene%20Component%20Object%20Reference) (bNewVisibility :type Boolean))
  (bind _output_get (Variables|Default|SetMarkerEnabled bNewVisibility))
  (Rendering|SetVisibility self2 _output_get false))