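; BP_Checkpoint is a checkpoint actor with a widget objective marker showing the player's distance in meters.
; BeginPlay applies MarkerEnabled to the widget's visibility, and while enabled, Tick updates the text through a lazily cached UI_Checkpoint reference.
; Any Sphere overlap hides the widget and spawns BP_Checkpoint1 at a hardcoded location, without filtering the actor, clearing MarkerEnabled or destroying itself.
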(event OnComponentBeginOverlap(Sphere)
  (params (OverlappedComponent :type Primitive%20Component%20Object%20Reference) (OtherActor :type Actor%20Object%20Reference) (OtherComp :type Primitive%20Component%20Object%20Reference) (OtherBodyIndex :type Integer) (bFromSweep :type Boolean) (SweepResult :type Hit%20Result%20Structure%20%28by%20ref%29))
  (Rendering|SetVisibility (Variables|Default|GetWidget) false false)
  (Game|SpawnActorfromClass "/Game/01_BluePrint/04_UI/BeeGameUI/BP_Checkpoint1.BP_Checkpoint1_C" (Math|Transform|MakeTransform "-16230.000000,-6000.000000,1500.000000" "0, 0, 0" "10.000000,10.000000,10.000000") "Undefined" "MultiplyWithRoot" 0 0))

(event EventBeginPlay
  (CallFunction|ToggleObjectiveMarker (Variables|Default|GetWidget) (Variables|Default|GetMarkerEnabled)))

(event Collision|EventActorBeginOverlap
  (params (OtherActor :type Actor%20Object%20Reference)))

(event EventTick
  (params (DeltaSeconds :type Float%20%28single-precision%29))
  (if (Variables|Default|GetMarkerEnabled)
    (CallFunction|UpdateDistance)))

(fn ConstructionScript)

(fn UpdateDistance
  (bind _as_ui_checkpoint (Variables|Default|GetAs%20UI%20Checkpoint)
    (:then
      _)
    (:else
      (bind _asui_checkpoint (Utilities|Casting|CastToUI_Checkpoint (UserInterface|GetUserWidgetObject (Variables|Default|GetWidget))))
      (Variables|Default|SetAs%20UI%20Checkpoint _asui_checkpoint)))
  (Default|UpdateText _as_ui_checkpoint (Utilities|Text|ToText(String) (Utilities|String|Append (Utilities|String|ToString(Integer) (Math|Float|Round (/ (Math|Vector|Distance(Vector) (Transformation|GetActorLocation (Game|GetPlayerCharacter 0)) (Transformation|GetActorLocation)) 1e+02))) "m"))))

(fn ToggleObjectiveMarker
  (params (self2 :type Scene%20Component%20Object%20Reference) (bNewVisibility :type Boolean))
  (bind _output_get (Variables|Default|SetMarkerEnabled bNewVisibility))
  (Rendering|SetVisibility self2 _output_get false))